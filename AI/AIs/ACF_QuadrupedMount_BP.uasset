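; ACF rideable quadruped mount that pawns interact with to mount or dismount; its own Interact input dismounts the rider.
; Sprint and brake inputs trigger rider actions through the mount component and hold a flag for the given duration.
; Tick reads these flags, sprint taking priority, and feeds acceleration or deceleration into the quadruped movement component's local forward movement.
; Acceleration also sets the sprint locomotion state.
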(event `self.ReceiveBeginPlay`
  (`parent.ReceiveBeginPlay`))

(event `ReceiveSprintInput`
  (params (Duration :type "Float (double-precision)"))
  (if (not (`self.Accelerating`))
    (set `self.Accelerating` true)
    (`ACFMountableComponent.TriggerActionOnRider` (`self.ACFMountComp`) (struct :`TagName` "Actions.HorseSprint") "ELow" false "")
    (`KismetSystemLibrary.RetriggerableDelay` Duration)
    (set `self.Accelerating` false)))

(event `self.ReceiveTick`
  (params (DeltaSeconds :type "Float (single-precision)"))
  (`parent.ReceiveTick` DeltaSeconds)
  (if (`self.Accelerating`)
    (`self.Accelerate` (`self.DefaultAccelleration`))
    (elif (`self.Braking`)
      (`self.Brake` (`self.DefaultDecel`)))))

(event `ReceiveBrakeInput`
  (params (Duration :type "Float (double-precision)"))
  (if (not (`self.Braking`))
    (set `self.Braking` true)
    (`ACFMountableComponent.TriggerActionOnRider` (`self.ACFMountComp`) (struct :`TagName` "Actions.HorseBreak") "ELow" false "")
    (`KismetSystemLibrary.RetriggerableDelay` Duration)
    (set `self.Braking` false)))

(event `InputAction|Interact`
  (params (Key :type "Key Structure"))
  (:`Pressed`
    (`ACFMountableComponent.TriggerActionOnRider` (`self.ACFMountComp`) (struct :`TagName` "Actions.Dismount") "ELow" false "")))

(event `ACFInteractableInterface.OnInteractedByPawn`
  (params (Pawn :type "Pawn Object Reference") (interactionType :type String))
  (bind _asacfcharacter (cast `ACFCharacter` Pawn))
  (if (`ACFMountComponent.IsMounted` (`self.ACFMountComp`))
    (`self.TriggerAction` _asacfcharacter (struct :`TagName` "Actions.Dismount") "ELow" false "")
    (else
      (`self.TriggerAction` _asacfcharacter (struct :`TagName` "Actions.Mount") "EHigh" false ""))))

(fn `Accelerate`
  (params (Value :type "Float (double-precision)"))
  (bind _asacfquadruped_movement_component (cast `ACFQuadrupedMovementComponent` (`self.LocomotionComp`)))
  (`ACFQuadrupedMovementComponent.MoveForwardLocal` _asacfquadruped_movement_component Value)
  (`ACFCharacterMovementComponent.SetLocomotionState` (`self.LocomotionComp`) "ESprint"))

(fn `Brake`
  (params (Value :type "Float (double-precision)"))
  (bind _asacfquadruped_movement_component (cast `ACFQuadrupedMovementComponent` (`self.LocomotionComp`)))
  (`ACFQuadrupedMovementComponent.MoveForwardLocal` _asacfquadruped_movement_component Value))

(fn `CanBeInteracted`
  (params (Pawn :type "Pawn Object Reference"))
  (returns (ReturnValue :type Boolean))
  (return true))

(fn `GetInteractableName`
  (returns (ReturnValue :type Text))
  (return (`self.GetCharacterName`)))

(fn `UserConstructionScript`
  (`parent.UserConstructionScript`))