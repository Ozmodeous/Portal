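; Parry action Blueprint for the ACF action system that lets a character parry hits and punish the attacker.
; It can run only when the owner's defense stance component allows parrying.
; Its sub-action state opens and closes the parry window, binding to damage-blocked events meanwhile.
; A block while parrying triggers a configured high-priority action on the damage dealer through its actions manager.
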(event `self.OnSubActionStateEntered`
  (bind _returnvalue (`Actor.GetComponentByClass` (`self.CharacterOwner`) "/Script/AscentCombatFramework.ACFDefenseStanceComponent"))
  ; Open Parry Window
  (`/Engine/EditorBlueprintResources/StandardMacros.IsValid` _returnvalue
    (:`Is Valid`
      (`ACFDefenseStanceComponent.StartParry` _returnvalue)
      (add `ACFDefenseStanceComponent.OnDamageBlocked` _returnvalue (delegate `CustomEvent`)))))

(event `CustomEvent`
  (params (blockedDamage :type "ACFDamageEvent Structure (by ref)"))
  (if (`ACFDefenseStanceComponent.IsParrying` (`Actor.GetComponentByClass` (`self.CharacterOwner`) "/Script/AscentCombatFramework.ACFDefenseStanceComponent"))
    (`ACFActionsManagerComponent.TriggerAction` (`Actor.GetComponentByClass` (`.DamageDealer` (break `ACFDamageEvent` blockedDamage)) "/Script/ActionsSystem.ACFActionsManagerComponent") (`self.ActionToBeTriggeredOnDamager`) "EHigh" false "")))

(event `self.OnSubActionStateExited`
  (bind _returnvalue (`Actor.GetComponentByClass` (`self.CharacterOwner`) "/Script/AscentCombatFramework.ACFDefenseStanceComponent"))
  ; Close Parry Window
  (`/Engine/EditorBlueprintResources/StandardMacros.IsValid` _returnvalue
    (:`Is Valid`
      (`ACFDefenseStanceComponent.StopParry` _returnvalue)
      (remove `ACFDefenseStanceComponent.OnDamageBlocked` _returnvalue (delegate `CustomEvent`)))))

(fn `CanExecuteAction`
  (params (owner :type "Character Object Reference"))
  (returns (ReturnValue :type Boolean))
  (bind _returnvalue (`Actor.GetComponentByClass` owner "/Script/AscentCombatFramework.ACFDefenseStanceComponent"))
  (`/Engine/EditorBlueprintResources/StandardMacros.IsValid` _returnvalue
    (:`Is Valid`
      (return (`ACFDefenseStanceComponent.CanParry` _returnvalue)))
    (:`Is Not Valid`
      (return false))))