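; ACF action Blueprint that makes a character fire its equipped ranged weapon at its current target.
; It can execute only when the owner's equipment component holds a ranged main weapon that reports it can shoot.
; When the action's notable point is reached, it calls ShootAtActor on that weapon with the character's target, a random deviation and an optional projectile override.
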(event `self.OnNotablePointReached`
  (`parent.OnNotablePointReached`)
  (bind _asacfcharacter (cast `ACFCharacter` (`self.CharacterOwner`)))
  (bind _asacfranged_weapon (cast `ACFRangedWeapon` (`ACFEquipmentComponent.GetCurrentMainWeapon` (`ACFCharacter.EquipmentComp` _asacfcharacter))))
  (`ACFRangedWeapon.ShootAtActor` _asacfranged_weapon (`ACFCharacter.GetTarget` _asacfcharacter) (`self.RandomDeviation`) 1.0 (`self.Projectile Override`)))

(fn `CanExecuteAction`
  (params (owner :type "Character Object Reference"))
  (returns (ReturnValue :type Boolean))
  (bind _returnvalue (`Actor.GetComponentByClass` owner "/Script/InventorySystem.ACFEquipmentComponent"))
  (`/Engine/EditorBlueprintResources/StandardMacros.IsValid` _returnvalue
    (:`Is Valid`
      (bind _asacfranged_weapon (cast `ACFRangedWeapon` (`ACFEquipmentComponent.GetCurrentMainWeapon` _returnvalue))
        (:`then`
          (return (`ACFRangedWeapon.CanShoot` _asacfranged_weapon)))
        (:`CastFailed`
          _)))
    (:`Is Not Valid`
      _))
  (return false))