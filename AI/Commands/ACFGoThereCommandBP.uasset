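; AI companion command that sends the AI to the point its lead actor is looking at.
; Line traces on Visibility from the lead's eye viewpoint along the view direction, using a camera offset and max distance, then runs AIMoveTo to the hit.
; Finishes successfully after a post-move delay, or fails on invalid lead, missed trace or failed move request.
; Debug drawing of the trace and hit sphere is left enabled.
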(event `self.ExecuteCommand`
  (params (controller :type "ACFAIController Object Reference"))
  (bind _returnvalue (`ACFAIController.GetLeadActorBK` controller))
  (bind (_outlocation _outrotation) (`Actor.GetActorEyesViewPoint` _returnvalue))
  (`/Engine/EditorBlueprintResources/StandardMacros.IsValid` _returnvalue
    (:`Is Valid`
      (bind (_outhit _returnvalue_2) (`KismetSystemLibrary.LineTraceSingle` _outlocation (+ (+ _outlocation (`self.CameraOffset`)) (* (`KismetMathLibrary.Conv_RotatorToVector` _outrotation) (`self.MaxDistance`))) "TraceTypeQuery1" true (`|MakeArray` _returnvalue) "Persistent"))
      (if _returnvalue_2
        (bind (_bblockinghit _binitialoverlap _time _distance _location) (`GameplayStatics.BreakHitResult` _outhit))
        (`KismetSystemLibrary.DrawDebugSphere` _location 100.0 12 (struct :`R` 1.0 :`G` 1.0 :`B` 1.0 :`A` 1.0) 5.0 5.0)
        (`AITask_MoveTo.AIMoveTo` (`self.GetAIController`) _location null
          (:`OnRequestFailed`
            (`self.FinishExecution` false))
          (:`OnMoveFinished`
            (`KismetSystemLibrary.Delay` (`self.Duration`))
            (`self.FinishExecution` true)))
        (else
          (`self.FinishExecution` false))))
    (:`Is Not Valid`
      (`self.FinishExecution` false))))