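; ACF overlap-volume component that lets its owning character automatically vault over or mantle onto nearby obstacles.
; It tracks overlapping actors and attempts a vault on each new overlap or on a retry timer while enabled, optionally only while falling.
; On authority, it traces candidates for edges and landing, passes results through ReplicateVariables, then triggers a vault action, or mantle as fallback, via the ACF actions manager.
; Getters expose the stored hits and vault distance.
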(event `self.ReceiveBeginPlay`
  (`parent.ReceiveBeginPlay`)
  (add `PrimitiveComponent.OnComponentBeginOverlap` (delegate `OnBeginOverlap`))
  (add `PrimitiveComponent.OnComponentEndOverlap` (`|CreateDelegate` :!event `OnEndOverlap`)))

(event `OnBeginOverlap`
  (params (OverlappedComponent :type "PrimitiveComponent Object Reference") (OtherActor :type "Actor Object Reference") (OtherComp :type "PrimitiveComponent Object Reference") (OtherBodyIndex :type Integer) (bFromSweep :type Boolean) (SweepResult :type "HitResult Structure (by ref)"))
  (if (!= (`self.GetOwner`) OtherActor)
    (`KismetArrayLibrary.Array_Add` (`self.OverlappingVaultables`) OtherActor)
    (`self.SetActorToVault` OtherActor)
    (`self.RetryOverlappingVaultables`)))

(event `OnEndOverlap`
  (params (OverlappedComponent :type "PrimitiveComponent Object Reference") (OtherActor :type "Actor Object Reference") (OtherComp :type "PrimitiveComponent Object Reference") (OtherBodyIndex :type Integer))
  (`KismetArrayLibrary.Array_RemoveItem` (`self.OverlappingVaultables`) OtherActor)
  (if (== OtherActor (`self.GetActorToVault`))
    (`self.SetActorToVault` null)))

(event `RetryOverlappingVaultables`
  (if (`self.ActivateOnlyWhenFalling`)
    (if (`NavMovementComponent.IsFalling` (`Character.CharacterMovement` (`self.GetCharacterOwner`)))
      (`self.TryToVaultActor`))
    (else
      (`self.TryToVaultActor`))))

(event `ReplicateVariables`
  (params (`Front Edge Hit` :type "HitResult Structure") (`Vaulting Orientation` :type "Vector Structure") (`Back Edge Hit` :type "HitResult Structure") (`Landing Hit` :type "HitResult Structure"))
  (set `self.Front Edge Hit` `Front Edge Hit`)
  (set `self.Vaulting Orientation` `Vaulting Orientation`)
  (set `self.Back Edge Hit` `Back Edge Hit`)
  (set `self.Landing Hit` `Landing Hit`))

(event `self.OnEnabledStateChanged`
  (params (bEnabled :type Boolean))
  ;[1 1 1] Enabling VaultChecks
  (if bEnabled
    (if (not (`KismetSystemLibrary.K2_IsValidTimerHandle` (`self.VaultRetryTimerHandle`)))
      (bind _returnvalue (`KismetSystemLibrary.K2_SetTimerDelegate` (`|CreateDelegate` :!event `RetryOverlappingVaultables`) (`self.RetryInterval_Seconds`) true))
      (set `self.VaultRetryTimerHandle` _returnvalue))
    (else
      (`KismetSystemLibrary.K2_InvalidateTimerHandle` (`self.VaultRetryTimerHandle`)))))

(fn `GetVaultDistance`
  (returns (ReturnValue :type "Float (double-precision)"))
  (bind (_front_edge_hit _vaulting_orientation _back_edge_hit) (`self.GetVaultValues`))
  (return (`KismetMathLibrary.VSize` (- (`.ImpactPoint` (`GameplayStatics.BreakHitResult` _front_edge_hit)) (`.ImpactPoint` (`GameplayStatics.BreakHitResult` _back_edge_hit))))))

(fn `GetVaultValues`
  (returns (`Front Edge Hit` :type "HitResult Structure") (`Vaulting Orientation` :type "Vector Structure") (`Back Edge Hit` :type "HitResult Structure") (`Landing Hit` :type "HitResult Structure"))
  (return (`self.Front Edge Hit`) (`self.Vaulting Orientation`) (`self.Back Edge Hit`) (`self.Landing Hit`)))

(fn `TryToVaultActor`
  (`/Engine/EditorBlueprintResources/ActorComponentMacros.Switch Has Authority`
    (:`Authority`
      (for _array_element (`self.OverlappingVaultables`)
        (`self.SetActorToVault` _array_element)
        (if (`self.CanVault`)
          (bind (_bvalid _frontedgehit _vaultingorientation _backedgehit _landinghit _validformantle) (`/AscentCombatFramework/CharacterController/ACF_VaultFunctionLibrary_BP.TraceOverlappingVaultable` (`self.GetCharacterOwner`) self (`self.GetActorToVault`) (`self.CharacterSpeedThreshold`) (`self.CharacterHeadingAngleThreshold`) (`self.VaultOverToMantleThreshold`) (`KismetMathLibrary.MakeVector2D` (`self.MinVaultOverFallDistance`) (`self.MaxVaultOverFallDistance`)) (`self.LandingClearanceBufferDistance`) (`self.Debug Draw`)))
          (if _bvalid
            (`self.ReplicateVariables` _frontedgehit _vaultingorientation _backedgehit _landinghit)
            (`ACFActionsManagerComponent.TriggerAction` (`Actor.GetComponentByClass` (`self.GetOwner`) "/Script/ActionsSystem.ACFActionsManagerComponent") (`self.GetVaultActionTag`) "EMedium" false "")
            (break)
            (elif (and _validformantle (`self.bCanMantle`))
              (`self.ReplicateVariables` _frontedgehit _vaultingorientation _backedgehit _landinghit)
              (`ACFActionsManagerComponent.TriggerAction` (`Actor.GetComponentByClass` (`self.GetOwner`) "/Script/ActionsSystem.ACFActionsManagerComponent") (struct :`TagName` "Actions.Mantle") "EMedium" false ""))))))))