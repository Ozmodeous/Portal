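; An ACF action that reloads the character's current ranged main weapon.
; It can execute only when allowed ammo is in the inventory and the magazine is not full.
; On start it saves and disables the anim instance's hand IK, then calls Reload on the weapon's shooting component.
; On end it restores the saved hand IK setting.
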(event `self.OnActionStarted`
  (params (contextString :type String))
  (`parent.OnActionStarted` contextString)
  (bind _asacfcharacter (cast `ACFCharacter` (`self.CharacterOwner`)))
  (set `self.OldEnabled` (`ACFAnimInstance.GetEnableHandIK` (`ACFCharacter.GetACFAnimInstance` _asacfcharacter)))
  (`self.EnableHandIK` false)
  (bind _equipmentcomp (`ACFCharacter.EquipmentComp` _asacfcharacter))
  (`/Engine/EditorBlueprintResources/StandardMacros.IsValid` _equipmentcomp
    (:`Is Valid`
      (bind _asacfranged_weapon (cast `ACFRangedWeapon` (`ACFEquipmentComponent.GetCurrentMainWeapon` _equipmentcomp)))
      (bind _returnvalue (`ACFRangedWeapon.GetShootingComponent` _asacfranged_weapon))
      (if (`.ReturnValue` (`ACFShootingComponent.TryGetAllowedAmmoFromInventory` _returnvalue))
        (`ACFShootingComponent.Reload` _returnvalue true)))))

(event `self.OnActionEnded`
  (`parent.OnActionEnded`)
  (`self.EnableHandIK` (`self.OldEnabled`)))

(fn `CanExecuteAction`
  (params (owner :type "Character Object Reference"))
  (returns (ReturnValue :type Boolean))
  (bind _asacfcharacter (cast `ACFCharacter` owner))
  (bind _equipmentcomp (`ACFCharacter.EquipmentComp` _asacfcharacter))
  (`/Engine/EditorBlueprintResources/StandardMacros.IsValid` _equipmentcomp
    (:`Is Valid`
      (bind _asacfranged_weapon (cast `ACFRangedWeapon` (`ACFEquipmentComponent.GetCurrentMainWeapon` _equipmentcomp))
        (:`then`
          (bind _returnvalue (`ACFRangedWeapon.GetShootingComponent` _asacfranged_weapon))
          (return (and (`.ReturnValue` (`ACFShootingComponent.TryGetAllowedAmmoFromInventory` _returnvalue)) (< (`ACFShootingComponent.GetCurrentAmmoInMagazine` _returnvalue) (`ACFShootingComponent.GetAmmoMagazine` _returnvalue)))))
        (:`CastFailed`
          _)))
    (:`Is Not Valid`
      _))
  (return false))

(fn `EnableHandIK`
  (params (val :type Boolean))
  (bind _asacfcharacter (cast `ACFCharacter` (`self.CharacterOwner`)))
  (`ACFAnimInstance.SetEnableHandIK` (`ACFCharacter.GetACFAnimInstance` _asacfcharacter) val))