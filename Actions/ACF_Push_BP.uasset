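; ACF push action that knocks the character's current target into a temporary ragdoll.
; At the action's notable point it reads the target from the ATS targeting component on the owner's controller.
; It applies an impulse at the pelvis along the owner-to-target direction through the target's ACF ragdoll component.
; The action can always execute, printing a debug message if the controller lacks a targeting component.
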(event `self.OnActionStarted`
  (params (contextString :type String))
  (`parent.OnActionStarted` contextString))

(event `self.OnNotablePointReached`
  (bind _characterowner (`self.CharacterOwner`))
  (bind _returnvalue (`Actor.GetComponentByClass` (`Pawn.GetController` _characterowner) "/Script/AscentTargetingSystem.ATSBaseTargetComponent"))
  (bind _returnvalue_2 (`ATSBaseTargetComponent.GetCurrentTarget` _returnvalue))
  (`/Engine/EditorBlueprintResources/StandardMacros.IsValid` _returnvalue
    (:`Is Valid`
      (`/Engine/EditorBlueprintResources/StandardMacros.IsValid` _returnvalue_2
        (:`Is Valid`
          (bind _output_get (set `self.Impulse` (make `RagdollImpulse` (`self.IImpulse Intensity`) (`KismetMathLibrary.GetForwardVector` (`KismetMathLibrary.FindLookAtRotation` (`Actor.K2_GetActorLocation` _characterowner) (`Actor.K2_GetActorLocation` _returnvalue_2))))))
          (`ACFRagdollComponent.GoRagdollForDuration` (`Actor.GetComponentByClass` _returnvalue_2 "/Script/AscentCombatFramework.ACFRagdollComponent") _output_get 5.0))))
    (:`Is Not Valid`
      (`KismetSystemLibrary.PrintString` "INVALID!!!"))))

(fn `CanExecuteAction`
  (params (owner :type "Character Object Reference"))
  (returns (ReturnValue :type Boolean))
  (return true))