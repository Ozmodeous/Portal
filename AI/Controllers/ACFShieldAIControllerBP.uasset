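; ACF AI controller for shield-bearing enemies that drives the controlled pawn's defense stance component.
; It raises defense when the AI state changes while in battle or the combat state becomes study target, and lowers it outside battle.
; On damage received, it also drops defense if the damage dealer's current action tag matches BreakDefenceWithTag, letting specific attacks break the guard.
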(event `self.ReceiveBeginPlay`
  (`parent.ReceiveBeginPlay`)
  (add `self.OnAIStateChanged` (delegate `OnCombatStarted`))
  (add `self.OnAICombatStateChanged` (delegate `OnAICombatStateChanged_Event_0`))
  (add `self.OnDamageReceived` (delegate `OnDamageReceived_Event`)))

(event `OnDamageReceived_Event` :!signature `self.OnDamageReceived`
  (params (damageReceived :type "ACFDamageEvent Structure (by ref)"))
  (bind _returnvalue (`self.GetDefenseComp`))
  ; BreakDefense
  (if (`KismetArrayLibrary.Array_Contains` (`BlueprintGameplayTagLibrary.BreakGameplayTagContainer` (`self.BreakDefenceWithTag`)) (`ACFActionsManagerComponent.GetCurrentActionTag` (`self.GetComponentByClass` (`.DamageDealer` (break `ACFDamageEvent` damageReceived)) "/Script/ActionsSystem.ACFActionsManagerComponent")))
    (`/Engine/EditorBlueprintResources/StandardMacros.IsValid` _returnvalue
      (:`Is Valid`
        (`ACFDefenseStanceComponent.StopDefending` _returnvalue)))))

(event `OnAICombatStateChanged_Event_0` :!signature `self.OnAICombatStateChanged`
  (params (AICombatState :type "EAICombatState Enum" :default "EMeleeCombat"))
  (bind _returnvalue (`self.GetDefenseComp`))
  ; StartDefense
  (if (`|EnumEquality` AICombatState "EStudyTarget")
    (`/Engine/EditorBlueprintResources/StandardMacros.IsValid` _returnvalue
      (:`Is Valid`
        (`ACFDefenseStanceComponent.StartDefending` _returnvalue)))))

(event `OnCombatStarted` :!signature `self.OnAIStateChanged`
  (params (AIState :type "GameplayTag Structure"))
  (bind _returnvalue (`self.GetDefenseComp`))
  (bind _returnvalue_2 (`self.GetDefenseComp`))
  ; StartDefense
  (if (`self.IsInBattle`)
    (`/Engine/EditorBlueprintResources/StandardMacros.IsValid` _returnvalue_2
      (:`Is Valid`
        (`ACFDefenseStanceComponent.StartDefending` _returnvalue_2)))
    (else
      (`/Engine/EditorBlueprintResources/StandardMacros.IsValid` _returnvalue
        (:`Is Valid`
          (`ACFDefenseStanceComponent.StopDefending` _returnvalue))))))

(fn `GetDefenseComp`
  (returns (ReturnValue :type "ACFDefenseStanceComponent Object Reference"))
  (return (`self.GetComponentByClass` (`self.K2_GetPawn`) "/Script/AscentCombatFramework.ACFDefenseStanceComponent")))

(fn `UserConstructionScript`
  (`parent.UserConstructionScript`))