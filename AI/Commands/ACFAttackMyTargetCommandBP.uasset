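; An AI group command in which a follower sets its target to whatever the group leader is attacking.
; It reads the group lead's current target, falling back to a single front trace from the leader's controller to find a character in front of it.
; The chosen target is set on the commanded controller and printed by name; the command fails without a group, a character lead or a found target.
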(event `self.ExecuteCommand`
  (params (controller :type "ACFAIController Object Reference"))
  (bind _returnvalue (`ACFAIController.GetGroup` controller))
  (bind _nexttarget (`self.NextTarget`))
  (set `self.Controller` controller)
  (`/Engine/EditorBlueprintResources/StandardMacros.IsValid` _returnvalue
    (:`Is Valid`
      (bind _asacfcharacter (cast `ACFCharacter` (`ACFGroupAIComponent.GetGroupLead` _returnvalue))
        (:`then`
          (bind _returnvalue_2 (`ACFCharacter.GetTarget` _asacfcharacter))
          (`/Engine/EditorBlueprintResources/StandardMacros.IsValid` _returnvalue_2
            (:`Is Valid`
              (set `self.NextTarget` _returnvalue_2)
              (`ACFAIController.SetTarget` (`self.Controller`) _nexttarget :!label _label)
              (`KismetSystemLibrary.PrintString` (`KismetSystemLibrary.GetDisplayName` _nexttarget))
              (`self.FinishExecution` true))
            (:`Is Not Valid`
              (bind _returnvalue_3 (`ACFFrontTracerComponent.PerformFrontTraceSingle` (`Actor.GetComponentByClass` (`Pawn.GetController` _asacfcharacter) "/Script/AscentCombatFramework.ACFFrontTracerComponent")))
              (bind _asacfcharacter_2 (cast `ACFCharacter` _returnvalue_3)
                (:`then`
                  (set `self.NextTarget` _asacfcharacter_2)
                  (goto _label))
                (:`CastFailed`
                  (`self.FinishExecution` false))))))
        (:`CastFailed`
          (`self.FinishExecution` false :!label _label_2))))
    (:`Is Not Valid`
      (goto _label_2))))