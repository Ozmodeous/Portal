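; ACF_OnHorseAttack_BP is an ACF action that performs a directional melee attack while the character is riding.
; It can execute only when the owner is an ACF character with a rider component, is riding, uses melee combat and passes the parent check.
; On start it stores the context string as the attack direction, which then selects the montage section to play.
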(event `self.OnActionStarted`
  (params (contextString :type String))
  (`parent.OnActionStarted` contextString)
  (set `self.AttackDirection` contextString))

(fn `CanExecuteAction`
  (params (owner :type "Character Object Reference"))
  (returns (ReturnValue :type Boolean))
  (bind _returnvalue (`Actor.GetComponentByClass` owner "/Script/MountSystem.ACFRiderComponent"))
  (`/Engine/EditorBlueprintResources/StandardMacros.IsValid` _returnvalue
    (:`Is Valid`
      (bind _asacfcharacter (cast `ACFCharacter` owner)
        (:`then`
          (switch `ECombatType` (`ACFCharacter.GetCombatType` _asacfcharacter)
            (:`EUnarmed`
              _)
            (:`EMelee`
              (bind _returnvalue_2 (`parent.CanExecuteAction` owner))
              (return (and _returnvalue_2 (`ACFRiderComponent.IsRiding` _returnvalue))))
            (:`ERanged`
              _)))
        (:`CastFailed`
          _)))
    (:`Is Not Valid`
      _))
  (return false))

(fn `GetMontageSectionName`
  (returns (ReturnValue :type Name))
  (return (`KismetStringLibrary.Conv_StringToName` (`self.AttackDirection`))))