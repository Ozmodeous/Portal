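; ACFDodgeActionBP is the dodge action for ACF characters, extending its parent action's start and end events.
; On start, it calls the parent, then disables foot IK on the character's ACF anim instance; on end, it calls the parent and re-enables it.
; A PlayerController cast at the end of the start event leads to no further logic.
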(event `self.OnActionStarted`
  (params (contextString :type String))
  (bind _characterowner (`self.CharacterOwner`))
  (`parent.OnActionStarted` contextString)
  (bind _asacfanim_instance (cast `ACFAnimInstance` (`SkeletalMeshComponent.GetAnimInstance` (`Character.Mesh` _characterowner))))
  (`ACFAnimInstance.SetEnableFootIK` _asacfanim_instance false)
  (cast `PlayerController` (`Pawn.GetController` _characterowner)))

(event `self.OnActionEnded`
  (`parent.OnActionEnded`)
  (bind _asacfanim_instance (cast `ACFAnimInstance` (`SkeletalMeshComponent.GetAnimInstance` (`Character.Mesh` (`self.CharacterOwner`)))))
  (`ACFAnimInstance.SetEnableFootIK` _asacfanim_instance true))