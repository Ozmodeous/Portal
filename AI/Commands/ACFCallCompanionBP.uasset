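; ACFCallCompanionBP is an AI command that calls a companion back to its lead actor.
; On execution it teleports the pawn near the lead if their distance is at least TeleportDistance.
; In either case it then runs an async AI Move To toward the lead, finishing the command as successful when the move finishes or as failed when the request fails.
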(event `self.ExecuteCommand`
  (params (controller :type "ACFAIController Object Reference"))
  (bind _output_get (set `self.Controller` controller))
  (if (>= (`Actor.GetDistanceTo` (`ACFAIController.GetLeadActorBK` _output_get) (`Controller.K2_GetPawn` _output_get)) (`self.TeleportDistance`))
    (`ACFAIController.TeleportNearLead` (`self.Controller`)))
  (`AITask_MoveTo.AIMoveTo` (`self.Controller`) (0.0 0.0 0.0) (`ACFAIController.GetLeadActorBK` (`self.Controller`))
    (:`OnRequestFailed`
      (`self.FinishExecution` false))
    (:`OnMoveFinished`
      (`self.FinishExecution` true))))