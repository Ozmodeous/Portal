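; ACFTauntActionBP is an ACF action that lets a character taunt its current target, drawing that target's aggro onto itself.
; When the action reaches its notable point, it runs the parent logic and takes the owning ACF character's target.
; If that target has an ACF AI controller, its threat manager gains ThreatToAdd threat toward the owner.
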(event `self.OnNotablePointReached`
  (`parent.OnNotablePointReached`)
  (bind _asacfcharacter (cast `ACFCharacter` (`self.CharacterOwner`)))
  (bind _returnvalue (`AIBlueprintHelperLibrary.GetAIController` (`ACFCharacter.GetTarget` _asacfcharacter)))
  (`/Engine/EditorBlueprintResources/StandardMacros.IsValid` _returnvalue
    (:`Is Valid`
      (bind _asacfaicontroller (cast `ACFAIController` _returnvalue))
      (`ACFThreatManagerComponent.AddThreat` (`ACFAIController.GetThreatManager` _asacfaicontroller) (`self.CharacterOwner`) (`self.ThreatToAdd`)))))