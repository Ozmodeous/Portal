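; Charged shot action for ACF ranged weapons such as bows, available only when the equipped main weapon can shoot.
; Starting it triggers a charge camera event and force feedback and pulls the bow string through the weapon's anim instance.
; On release, clamped hold time becomes the charge, firing at the local controller's current target or falling back to an untargeted projectile.
; Releases below minimum charge stop the action without firing.
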(event `self.OnActionReleased`
  (params (elapsedTimeSeconds :type "Float (single-precision)"))
  (bind _asacfbow_anim_instance (`self.GetBowABP`))
  (bind _returnvalue (`Actor.GetComponentByClass` (`self.CharacterOwner`) "/Script/InventorySystem.ACFEquipmentComponent"))
  (bind _returnvalue_2 (`Actor.GetComponentByClass` (`ACFFunctionLibrary.GetLocalACFPlayerController`) "/Script/AscentTargetingSystem.ATSBaseTargetComponent"))
  (bind _returnvalue_3 (`ATSBaseTargetComponent.GetCurrentTarget` _returnvalue_2))
  (bind _output_get (set `self.FinalCharge` (`KismetMathLibrary.FClamp` elapsedTimeSeconds 0.0 (`self.MaxCharge`))))
  (if (>= _output_get (`self.MinCharge`))
    (`|ExecutionSequence`
      (:`then_0`
        (`/Engine/EditorBlueprintResources/StandardMacros.IsValid` _returnvalue
          (:`Is Valid`
            (bind _asacfranged_weapon (cast `ACFRangedWeapon` (`ACFEquipmentComponent.GetCurrentMainWeapon` _returnvalue)))
            (set `self.CurrentWeapon` _asacfranged_weapon)
            (`/Engine/EditorBlueprintResources/StandardMacros.IsValid` _returnvalue_2
              (:`Is Valid`
                (`/Engine/EditorBlueprintResources/StandardMacros.IsValid` _returnvalue_3
                  (:`Is Valid`
                    (`ACFRangedWeapon.ShootAtActor` (`self.CurrentWeapon`) _returnvalue_3 2.0 (`self.FinalCharge`) (`self.Projectile Override`)))
                  (:`Is Not Valid`
                    (`ACFRangedWeapon.ShootProjectile` (`self.CurrentWeapon`) (`self.Target Type`) (`self.FinalCharge`) (`self.Projectile Override`) :!label _label))))
              (:`Is Not Valid`
                (goto _label))))))
      (:`then_1`
        (`CCMCameraFunctionLibrary.StopCameraEvent` (`self.ChargeCameraEvent`) :!label _label_2)
        (`/Engine/EditorBlueprintResources/StandardMacros.IsValid` _asacfbow_anim_instance
          (:`Is Valid`
            (`ACFBowAnimInstance.ReleaseString` _asacfbow_anim_instance)))))
    (else
      (`self.StopActionImmediately`)
      (goto _label_2))))

(event `self.ClientsOnActionStarted`
  (params (contextString :type String))
  (bind _asacfbow_anim_instance (`self.GetBowABP`))
  (`CCMCameraFunctionLibrary.TriggerCameraEvent` (`self.ChargeCameraEvent`))
  (`GameplayStatics.SpawnForceFeedbackAttached` (`self.Force Feedback Effect`) (`Character.Mesh` (`self.CharacterOwner`)) "None" (0.0 0.0 0.0) (struct) "KeepRelativeOffset" false false 1.0 0.0 null)
  (`/Engine/EditorBlueprintResources/StandardMacros.IsValid` _asacfbow_anim_instance
    (:`Is Valid`
      (`ACFBowAnimInstance.PullString` _asacfbow_anim_instance))))

(event `self.ClientsOnActionEnded`
  (`CCMCameraFunctionLibrary.StopCameraEvent` (`self.ChargeCameraEvent`)))

(event `self.OnTick`
  (params (DeltaTime :type "Float (single-precision)"))
  (`KismetSystemLibrary.PrintString` (`KismetStringLibrary.Conv_DoubleToString` (`GameplayStatics.GetRealTimeSeconds`)) true true (struct :`G` 0.66 :`B` 1.0 :`A` 1.0) 0.0))

(fn `CanExecuteAction`
  (params (owner :type "Character Object Reference"))
  (returns (ReturnValue :type Boolean))
  (bind _returnvalue (`Actor.GetComponentByClass` owner "/Script/InventorySystem.ACFEquipmentComponent"))
  (`/Engine/EditorBlueprintResources/StandardMacros.IsValid` _returnvalue
    (:`Is Valid`
      (bind _asacfranged_weapon (cast `ACFRangedWeapon` (`ACFEquipmentComponent.GetCurrentMainWeapon` _returnvalue))
        (:`then`
          (return (`ACFRangedWeapon.CanShoot` _asacfranged_weapon)))
        (:`CastFailed`
          _)))
    (:`Is Not Valid`
      _))
  (return false))

(fn `GetBowABP`
  (returns (`AsACFBow Anim Instance` :type "ACFBowAnimInstance Object Reference"))
  (bind _returnvalue (`Actor.GetComponentByClass` (`self.CharacterOwner`) "/Script/InventorySystem.ACFEquipmentComponent"))
  (bind _returnvalue_2 (`ACFEquipmentComponent.GetCurrentMainWeapon` _returnvalue))
  (bind _returnvalue_3 (`ACFWeapon.GetMeshComponent` _returnvalue_2))
  (`/Engine/EditorBlueprintResources/StandardMacros.IsValid` _returnvalue
    (:`Is Valid`
      (`/Engine/EditorBlueprintResources/StandardMacros.IsValid` _returnvalue_2
        (:`Is Valid`
          (`/Engine/EditorBlueprintResources/StandardMacros.IsValid` _returnvalue_3
            (:`Is Valid`
              (bind _asacfbow_anim_instance (cast `ACFBowAnimInstance` (`SkeletalMeshComponent.GetAnimInstance` _returnvalue_3)))
              (return _asacfbow_anim_instance))))))))